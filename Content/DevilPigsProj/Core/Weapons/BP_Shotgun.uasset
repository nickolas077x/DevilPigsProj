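; Shotgun weapon Blueprint with a flipbook sprite that fires a spread of hitscan pellets.
; Fire plays the shoot flipbook, then runs one Visibility line trace per fraction and applies damage to each hit actor.
; RF0 rerolls random roll and yaw offsets within the spread, which rotate the end location vector for each trace.
; Traces draw timed debug lines, and the impact emitter is never run.
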(fn `Fire`
  (params (StartLocation :type "Vector Structure") (EndLocation :type "Vector Structure"))
  (`PaperFlipbookComponent.SetFlipbook` (`self.GunSprite`) (`self.FB_Shoot`))
  (`self.RF_0`)
  (for _ (range (+ (`self.Fractions`) 1))
    (`self.RF_0`)
    (bind (_outhit _returnvalue) (`KismetSystemLibrary.LineTraceSingle` :`Start` StartLocation :`End` (`KismetMathLibrary.GreaterGreater_VectorRotator` EndLocation (`KismetMathLibrary.MakeRotator` (`self.RandFloatY_0`) 0.0 (`self.RandFloatZ_0`))) :`TraceChannel` "TraceTypeQuery1" :`DrawDebugType` "ForDuration" :`DrawTime` 0.5))
    (if _returnvalue
      (`GameplayStatics.ApplyDamage` (`.HitActor` (`GameplayStatics.BreakHitResult` _outhit)) (`self.Damage`) null self))))

(fn `RF_0`
  (bind _spreadindegrees_0 (`self.SpreadInDegrees_0`))
  (bind _spreadindegrees_0_2 (`self.SpreadInDegrees_0`))
  (set `self.RandFloatY_0` (- (`KismetMathLibrary.RandomFloatInRange` 0.0 _spreadindegrees_0_2) (/ _spreadindegrees_0_2 2.0)))
  (set `self.RandFloatZ_0` (- (`KismetMathLibrary.RandomFloatInRange` 0.0 _spreadindegrees_0) (/ _spreadindegrees_0 2.0))))

(fn `UserConstructionScript`
  (`parent.UserConstructionScript`))