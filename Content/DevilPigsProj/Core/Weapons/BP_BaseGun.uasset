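; BP_BaseGun is a base hitscan gun that uses flipbook sprites for idle, shoot and reload animations.
; Fire randomizes spread through RF, rotates the EndLocation vector by it, then runs a debug-drawn Visibility line trace.
; Only a hit spawns an emitter, switches to the shoot flipbook and applies damage.
; Non-looping animations return to Idle on finishing; Reload is animation-only, and Show and Hide are empty stubs.
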(event `self.ReceiveBeginPlay`
  (`PaperFlipbookComponent.SetLooping` (`self.GunSprite`) false))

(event `self.GunSprite.OnFinishedPlaying`
  (`self.Idle`))

(fn `Fire`
  (params (StartLocation :type "Vector Structure") (EndLocation :type "Vector Structure"))
  (`self.RF`)
  (bind (_outhit _returnvalue) (`KismetSystemLibrary.LineTraceSingle` :`Start` StartLocation :`End` (`KismetMathLibrary.GreaterGreater_VectorRotator` EndLocation (`KismetMathLibrary.MakeRotator` (`self.RandFloatY`) 0.0 (`self.RandFloatZ`))) :`TraceChannel` "TraceTypeQuery1" :`DrawDebugType` "ForDuration"))
  (if _returnvalue
    (bind (_bblockinghit _binitialoverlap _time _distance _location _impactpoint _normal _impactnormal _physmat _hitactor) (`GameplayStatics.BreakHitResult` _outhit))
    (`GameplayStatics.SpawnEmitterAtLocation` null _location)
    (`PaperFlipbookComponent.SetFlipbook` (`self.GunSprite`) (`self.FB_Shoot`))
    (`GameplayStatics.ApplyDamage` _hitactor (`self.Damage`) null self)))

(fn `Hide`)

(fn `Idle`
  (bind _gunsprite (`self.GunSprite`))
  (`PaperFlipbookComponent.SetFlipbook` _gunsprite (`self.FB_Idle`))
  (`PaperFlipbookComponent.PlayFromStart` _gunsprite))

(fn `Reload`
  (bind _gunsprite (`self.GunSprite`))
  (`PaperFlipbookComponent.SetFlipbook` _gunsprite (`self.FB_Reload`))
  (`PaperFlipbookComponent.PlayFromStart` _gunsprite))

(fn `RF`
  (bind _spreadindegrees (`self.SpreadInDegrees`))
  (bind _spreadindegrees_2 (`self.SpreadInDegrees`))
  (set `self.RandFloatY` (- (`KismetMathLibrary.RandomFloatInRange` 0.0 _spreadindegrees_2) (/ _spreadindegrees_2 2.0)))
  (set `self.RandFloatZ` (- (`KismetMathLibrary.RandomFloatInRange` 0.0 _spreadindegrees) (/ _spreadindegrees 2.0)))
  (return))

(fn `Show`)

(fn `UserConstructionScript`)