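; First-person player character with axis-driven movement and look that spawns a BP_Shotgun on BeginPlay and attaches it at GunLocation.
; Fire traces a start and end point from the camera's forward vector and passes them to the equipped gun.
; A CanShoot flag and the gun's FireRate gate shots, with automatic guns re-firing by timer while the button is held.
; Reload calls the gun and briefly blocks shooting for that same interval.
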(event `self.ReceiveTick`
  (params (DeltaSeconds :type "Float (single-precision)")))

(event `InputAction|Fire`
  (params (Key :type "Key Structure"))
  (:`Pressed`
    (set `self.ShootButtonPressed` true)
    (`self.Fire`))
  (:`Released`
    (set `self.ShootButtonPressed` false)))

(event `InputAxis|MoveForward`
  (params (AxisValue :type "Float (single-precision)"))
  (`self.AddMovementInput` (`self.GetActorForwardVector`) AxisValue))

(event `InputAxis|LookUp`
  (params (AxisValue :type "Float (single-precision)"))
  (`self.AddControllerPitchInput` AxisValue))

(event `Fire`
  (bind _fpscamera (`self.FPSCamera`))
  (bind _returnvalue (`SceneComponent.K2_GetComponentLocation` _fpscamera))
  (bind _firerate (`/Game/DevilPigsProj/Core/Weapons/BP_BaseGun.FireRate` (`self.EquippedGun`)))
  (if (`self.ShootButtonPressed`)
    (if (`self.CanShoot`)
      (`/Game/DevilPigsProj/Core/Weapons/BP_BaseGun.Fire` (`self.EquippedGun`) _returnvalue (+ _returnvalue (* (`SceneComponent.GetForwardVector` _fpscamera) (`/Game/DevilPigsProj/Core/Weapons/BP_BaseGun.MaxBulletDistance` (`self.EquippedGun`)))))
      (set `self.CanShoot` false)
      (if (`/Game/DevilPigsProj/Core/Weapons/BP_BaseGun.IsAuto` (`self.EquippedGun`))
        (`KismetSystemLibrary.K2_SetTimerDelegate` (delegate `Fire`) _firerate)
        (else
          (`KismetSystemLibrary.Delay` _firerate)))
      (set `self.CanShoot` true))))

(event `InputAxis|MoveRight`
  (params (AxisValue :type "Float (single-precision)"))
  (`self.AddMovementInput` (`self.GetActorRightVector`) AxisValue))

(event `InputAxis|Turn`
  (params (AxisValue :type "Float (single-precision)"))
  (`self.AddControllerYawInput` AxisValue))

(event `self.ReceiveBeginPlay`
  (bind _returnvalue (`|SpawnActorFromClass` "/Game/DevilPigsProj/Core/Weapons/BP_Shotgun.BP_Shotgun_C" (`KismetMathLibrary.MakeTransform` (0.0 0.0 0.0)) "Undefined" "OverrideRootScale" null null))
  (bind _output_get (set `self.EquippedGun` _returnvalue))
  (`self.K2_AttachToComponent` _output_get (`self.GunLocation`) "None" "SnapToTarget" "SnapToTarget" "KeepRelative" true))

(event `InputAction|Reload`
  (params (Key :type "Key Structure"))
  (:`Pressed`
    (`/Game/DevilPigsProj/Core/Weapons/BP_BaseGun.Reload` (`self.EquippedGun`))
    (set `self.CanShoot` false)
    (`KismetSystemLibrary.Delay` (`/Game/DevilPigsProj/Core/Weapons/BP_BaseGun.FireRate` (`self.EquippedGun`)))
    (set `self.CanShoot` true)))

(fn `UserConstructionScript`)